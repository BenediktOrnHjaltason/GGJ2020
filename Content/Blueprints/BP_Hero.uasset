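; BP_Hero is the player hero Blueprint that sets up the HUD and opens the crafting menu.
; On BeginPlay it creates the HUD widget, adds it to the viewport and passes itself as HeroRef.
; The OpenCraftingMenu input creates a crafting menu widget with the same back-reference, then disables player controller input and shows the mouse cursor.
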(event EventBeginPlay
  (bind _returnvalue (UserInterface|CreateWidget "/Game/Blueprints/Widgets/HUD.HUD_C"))
  (UserInterface|Viewport|AddtoViewport _returnvalue 0)
  (Variables|/Game/Blueprints/Widgets/HUD.HUD_C|SetHeroRef _returnvalue self))

(event Collision|EventActorBeginOverlap
  (params (OtherActor :type Actor%20Object%20Reference)))

(event EventTick
  (params (DeltaSeconds :type Float%20%28single-precision%29)))

(event Input|ActionEvents|InputActionOpenCraftingMenu
  (params (Key :type Key%20Structure :default "None"))
  (bind _returnvalue (Game|GetPlayerController 0))
  (:Pressed
    (bind _returnvalue_2 (UserInterface|CreateWidget "/Game/Blueprints/Widgets/W_CraftingMenu.W_CraftingMenu_C"))
    (UserInterface|Viewport|AddtoViewport _returnvalue_2 0)
    (Variables|/Game/Blueprints/Widgets/W_CraftingMenu.W_CraftingMenu_C|SetHeroRef _returnvalue_2 self)
    (Input|DisableInput _returnvalue 0)
    (Variables|/Script/Engine.PlayerController|SetbShowMouseCursor _returnvalue true)))

(fn ConstructionScript)