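; BlockSpawnerMenu is a constantly spinning spawner actor that flings BP_Block actors, likely as a menu decoration given its name.
; Tick rotates it rapidly in yaw, so each block's impulse along the right vector follows the current facing.
; Nested looping timers fire bursts: one periodically starts per-second SpawnBlock calls, and a counter clears that timer after four blocks.
; BeginPlay also triggers the first burst immediately.
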(event EventBeginPlay
  (CallFunction|StartSpawning)
  (CallFunction|Spawn4Blocks))

(event Collision|EventActorBeginOverlap
  (params (OtherActor :type Actor%20Object%20Reference)))

(event EventTick
  (params (DeltaSeconds :type Float%20%28single-precision%29))
  (Class|Actor|AddActorWorldRotation (Math|Rotator|MakeRotator 0.0 0.0 (* DeltaSeconds 6e+02))))

(fn ConstructionScript)

(fn SpawnBlock
  (bind _returnvalue (Game|SpawnActorfromClass "/Game/Blueprints/BP_Block.BP_Block_C" (Transformation|GetActorTransform) "Undefined" 0 0))
  (Physics|AddImpulse (Variables|/Script/GGJ2020.Block|GetMesh _returnvalue) (* (Transformation|GetActorRightVector) 1.3e+05) "None" false)
  (bind _result (Math|Integer|IncrementInt (Variables|Default|GetSpawnCounter))
    (:%20%20
      (Math|Integer|CompareInt _result 4
        (:==
          (Utilities|Time|ClearTimerbyFunctionName 0 "SpawnBlock")
          (Variables|Default|SetSpawnCounter 0))))))

(fn Spawn4Blocks
  (Utilities|Time|SetTimerbyFunctionName 0 "SpawnBlock" 1.0 true))

(fn StartSpawning
  (Utilities|Time|SetTimerbyFunctionName 0 "Spawn4Blocks" 6.0 true))